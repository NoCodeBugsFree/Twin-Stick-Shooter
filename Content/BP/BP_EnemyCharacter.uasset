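; Enemy character Blueprint for a twin-stick game, with a health bar widget and a tinted body.
; BeginPlay passes the widget's progress bar to SetProgressBarReference, and construction applies EnemyColor through a dynamic material instance.
; AffectHealth is an empty event; the death, scoring, explosion and timed hero-attack chains are disconnected and never run.
; DamegeTheHero applies Damage to Hero, but only a disconnected chain sets its timer.
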(event `/Game/BP/I_Damageble.AffectHealth`
  (params (Delta :type "Float (single-precision)")))

(event `DamegeTheHero`
  (`/Game/BP/BP_HeroCharacter.AffectHealth` (`self.Hero`) (`self.Damage`)))

(event `self.ReceiveBeginPlay`
  ;[1 1 1] Set Health Bar Reference
  (bind _asbp_health_widget_cpp (cast `/Game/BP/BP_HealthWidgetCPP` (`WidgetComponent.GetUserWidgetObject` (`self.HealthBarWidget`))))
  (`self.SetProgressBarReference` (`/Game/BP/BP_HealthWidgetCPP.HealthBar` _asbp_health_widget_cpp)))

(fn `UserConstructionScript`
  (bind _returnvalue (`PrimitiveComponent.CreateDynamicMaterialInstance` (`self.Mesh`) 0 null))
  (bind _output_get (set `self.EnemyMaterial` _returnvalue))
  (`MaterialInstanceDynamic.SetVectorParameterValue` _output_get "BodyColor" (`self.EnemyColor`)))