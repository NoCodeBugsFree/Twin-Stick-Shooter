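; Player hero character Blueprint for a twin-stick game; its only live event logic hooks up the health bar.
; On BeginPlay it casts the HealthBarWidget component's widget to BP_HealthWidgetCPP and passes its HealthBar to SetProgressBarReference.
; Disconnected leftovers remain for HUD creation, weapon attachment, spawn-transform saving and aim rotation, the last using the CheckShouldFire rotation-comparison helper.
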(event `self.ReceiveBeginPlay`
  ;[0.124 0.6299 1] Set Health Bar Reference
  (bind _asbp_health_widget_cpp (cast `/Game/BP/BP_HealthWidgetCPP` (`WidgetComponent.GetUserWidgetObject` (`self.HealthBarWidget`))))
  (`self.SetProgressBarReference` (`/Game/BP/BP_HealthWidgetCPP.HealthBar` _asbp_health_widget_cpp)))

(fn `CheckShouldFire`
  (params (CurrentRotation :type "Rotator Structure") (DesiredRotation :type "Rotator Structure"))
  (returns (ShouldFire :type Boolean))
  (return (== CurrentRotation DesiredRotation :`ErrorTolerance` 0.1)))

(fn `UserConstructionScript`)